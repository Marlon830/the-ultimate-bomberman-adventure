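; Bomb actor that, once spawned, plays a scaling timeline as a fuse, then explodes in a cross along the world X and Y axes.
; Each arm is a single box trace that destroys the first object hit if it is a BP_BreakableWall, with debug drawing on.
; An active range power-up tints the bomb pink and overrides Range.
; After exploding, it destroys itself and increments the Player's BombCounter.
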(event `self.ReceiveBeginPlay`
  (bind _bomb (`self.Bomb`))
  (bind _player (`self.Player`))
  (bind _range (`self.Range`))
  (bind _israngepowerupactive (`self.IsRangePowerUpActive`))
  (bind _returnvalue (`SceneComponent.K2_GetComponentLocation` (`self.Bomb`)))
  (if _israngepowerupactive
    (`PrimitiveComponent.SetMaterial` (`self.Bomb`) 0 "/Game/Materials/M_ColorPink.M_ColorPink")
    (bind (_direction _newtrack_0) (`Timeline|Timeline` :!via `PlayFromStart` :!label _label)
      (:`Update`
        (`SceneComponent.K2_SetWorldTransform` _bomb (`KismetMathLibrary.MakeTransform` (`SceneComponent.K2_GetComponentLocation` _bomb) (struct) (`KismetMathLibrary.Conv_DoubleToVector` _newtrack_0)) false false))
      (:`Finished`
        (if _israngepowerupactive
          (set `self.Range` 300.0))
        (`self.ExplodeInAllDirections` (`KismetMathLibrary.MakeVector` _range) (+ _returnvalue (100.0 0.0 0.0)))
        (`self.ExplodeInAllDirections` (`KismetMathLibrary.MakeVector` (* _range -1.0)) (+ _returnvalue (-100.0 0.0 0.0)))
        (`self.ExplodeInAllDirections` (`KismetMathLibrary.MakeVector` 0.0 _range) (+ _returnvalue (0.0 100.0 0.0)))
        (`self.ExplodeInAllDirections` (`KismetMathLibrary.MakeVector` 0.0 (* _range -1.0)) (+ _returnvalue (0.0 -100.0 0.0)))
        (`self.K2_DestroyActor`)
        (set `/Game/ThirdPerson/Blueprints/BP_ThirdPersonCharacter.BombCounter` (+ 1 (`/Game/ThirdPerson/Blueprints/BP_ThirdPersonCharacter.BombCounter` _player)) _player)))
    (else
      (goto _label :!via `PlayFromStart`))))

(fn `ExplodeInAllDirections`
  (params (Direction :type "Vector Structure") (Start :type "Vector Structure"))
  (bind (_outhit _returnvalue) (`KismetSystemLibrary.BoxTraceSingleForObjects` :`Start` Start :`End` (+ Start Direction) :`HalfSize` (30.0 30.0 30.0) :`ObjectTypes` (`|MakeArray` "ObjectTypeQuery7" "ObjectTypeQuery8" :!type "EObjectTypeQuery Enum") :`DrawDebugType` "ForDuration"))
  (cast `/Game/Blueprints/BP_BreakableWall` (`.HitActor` (`GameplayStatics.BreakHitResult` _outhit)))
  (if _returnvalue
    (`self.K2_DestroyActor` (`.HitActor` (`GameplayStatics.BreakHitResult` _outhit)))))

(fn `UserConstructionScript`)